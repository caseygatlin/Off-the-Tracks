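; Rail trigger that marks an obstacle on any combination of left, center and right for the player's mine cart.
; When triggered, it casts the carriage to BP_Player_MineCart and passes the three flags to ProcessObstacle, ignoring other carriages.
; The construction script sets three editor indicator sprites to marked or blank to show which positions are flagged.
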(event EventInternalTriggerEvent
  (params (Bogie :type AC%20Bogie%20Object%20Reference) (Carriage :type BP%20Train%20Carriage%20Object%20Reference))
  (bind _asbp_player_mine_cart (Utilities|Casting|CastToBP_Player_MineCart Carriage))
  (Default|ProcessObstacle _asbp_player_mine_cart (Variables|Default|GetLeft) (Variables|Default|GetCenter) (Variables|Default|GetRight) 0.0))

(fn ConstructionScript
  (|CallParentFunction)
  (bind _newparam (CallFunction|GetEditorIndicatorSprite (Variables|Default|GetLeft)))
  (Rendering|Components|Sprite|SetSprite (Variables|Default|GetEditorLeft) _newparam)
  (bind _newparam_2 (CallFunction|GetEditorIndicatorSprite (Variables|Default|GetCenter)))
  (Rendering|Components|Sprite|SetSprite (Variables|Default|GetEditorCenter) _newparam_2)
  (bind _newparam_3 (CallFunction|GetEditorIndicatorSprite (Variables|Default|GetRight)))
  (Rendering|Components|Sprite|SetSprite (Variables|Default|GetEditorRight) _newparam_3))

(fn GetEditorIndicatorSprite
  (params (IndicatorState :type Boolean))
  (if IndicatorState
    (return "/Game/HandCarContent/Textures/MarkedIndicator_Sprite.MarkedIndicator_Sprite")
    (else
      (return "/Game/HandCarContent/Textures/BlankIndicator_Sprite.BlankIndicator_Sprite"))))