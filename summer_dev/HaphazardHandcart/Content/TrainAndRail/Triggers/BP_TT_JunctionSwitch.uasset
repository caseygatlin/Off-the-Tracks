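; Train track trigger that switches a junction by changing which connection is active on a target track.
; When the trigger fires, it sets the track's end or start active connection to a new one, with a flag choosing which end.
; On trigger reset it can optionally apply a separate reset connection to that same end, if one is valid.
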(event EventBeginPlay)

(event Collision|EventActorBeginOverlap
  (params (OtherActor :type Actor%20Object%20Reference)))

(event EventInternalTriggerEvent
  (params (Bogie :type AC%20Bogie%20Object%20Reference) (Carriage :type BP%20Train%20Carriage%20Object%20Reference))
  (Utilities|IsValid (Variables|SwitchOptions|GetTrackToUpdate)
    (:Is%20Valid
      (if (Variables|SwitchOptions|GetApplyActiveConnectionToEOT)
        (Variables|/Game/TrainAndRail/Blueprints/BP_TrainTrack.BP_TrainTrack_C|SetEnd_ActiveConnection (Variables|SwitchOptions|GetTrackToUpdate) (Variables|SwitchOptions|GetNewActiveConnection))
        (else
          (Variables|/Game/TrainAndRail/Blueprints/BP_TrainTrack.BP_TrainTrack_C|SetStart_ActiveConnection (Variables|SwitchOptions|GetTrackToUpdate) (Variables|SwitchOptions|GetNewActiveConnection)))))))

(event EventTick
  (params (DeltaSeconds :type Float%20%28single-precision%29))
  (|CallParentFunction 0.0))

(event EventPostTriggerResetEvent
  (if (Variables|SwitchOptions|GetRestTrackOnTriggerRest)
    (Utilities|IsValid (Variables|SwitchOptions|GetResetActiveConnection)
      (:Is%20Valid
        (if (Variables|SwitchOptions|GetApplyActiveConnectionToEOT)
          (Variables|/Game/TrainAndRail/Blueprints/BP_TrainTrack.BP_TrainTrack_C|SetEnd_ActiveConnection (Variables|SwitchOptions|GetTrackToUpdate) (Variables|SwitchOptions|GetResetActiveConnection))
          (else
            (Variables|/Game/TrainAndRail/Blueprints/BP_TrainTrack.BP_TrainTrack_C|SetStart_ActiveConnection (Variables|SwitchOptions|GetTrackToUpdate) (Variables|SwitchOptions|GetResetActiveConnection))))))))

(fn ConstructionScript
  (|CallParentFunction))