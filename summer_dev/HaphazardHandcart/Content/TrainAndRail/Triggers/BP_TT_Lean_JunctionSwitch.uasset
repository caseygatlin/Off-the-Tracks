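; BP_TT_Lean_JunctionSwitch is a track trigger that lets the player steer a junction by leaning the mine cart.
; On trigger, it casts the carriage to BP_Player_MineCart and sets the track's end active connection to the left, center or right track based on the cart's lean state.
; Its construction script turns on active-connection use at the end of the assigned track.
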(event EventInternalTriggerEvent
  (params (Bogie :type AC%20Bogie%20Object%20Reference) (Carriage :type BP%20Train%20Carriage%20Object%20Reference))
  (Utilities|IsValid (Variables|Default|GetTrack)
    (:Is%20Valid
      (bind _asbp_player_mine_cart (Utilities|Casting|CastToBP_Player_MineCart Carriage))
      (switch Utilities|FlowControl|Switch|SwitchonCartLeanState (Variables|/Game/TrainAndRail/Trains/BP_Player_MineCart.BP_Player_MineCart_C|GetCartLeanState _asbp_player_mine_cart)
        (:NewEnumerator3
          (Variables|/Game/TrainAndRail/Blueprints/BP_TrainTrack.BP_TrainTrack_C|SetEnd_ActiveConnection (Variables|Default|GetTrack) (Variables|SwitchOptions|GetLeftTrack)))
        (:NewEnumerator4
          (Variables|/Game/TrainAndRail/Blueprints/BP_TrainTrack.BP_TrainTrack_C|SetEnd_ActiveConnection (Variables|Default|GetTrack) (Variables|SwitchOptions|GetCenterTrack)))
        (:NewEnumerator5
          (Variables|/Game/TrainAndRail/Blueprints/BP_TrainTrack.BP_TrainTrack_C|SetEnd_ActiveConnection (Variables|Default|GetTrack) (Variables|SwitchOptions|GetRightTrack)))))))

(fn ConstructionScript
  (|CallParentFunction)
  (Utilities|IsValid (Variables|Default|GetTrack)
    (:Is%20Valid
      (Variables|/Game/TrainAndRail/Blueprints/BP_TrainTrack.BP_TrainTrack_C|SetEnd_UseActiveConnection (Variables|Default|GetTrack) true))))