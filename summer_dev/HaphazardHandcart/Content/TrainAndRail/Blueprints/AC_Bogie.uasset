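; Bogie component that tracks a train bogie's position along track splines in a train and rail system.
; ChangeTrack binds it to a track spline, and TickMovement advances its distance by speed, honoring inverted travel direction.
; GetTransform samples the spline, yawed 180 degrees when inverted, while other queries report the track end ahead and its connection points.
; An update ID lets RestorePreviousDistance undo the matching move.
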(event EventBeginPlay)

(event EventTick
  (params (DeltaSeconds :type Float%20%28single-precision%29)))

(fn ChangeTrack
  (params (Track :type BP%20Train%20Track%20Object%20Reference) (TrackSplineIndex :type Integer) (DistanceOnTrack :type Float%20%28single-precision%29))
  (bind _tracksplines (Variables|/Game/TrainAndRail/Blueprints/BP_TrainTrack.BP_TrainTrack_C|GetTrackSplines Track))
  (bind _returnvalue (Utilities|Array|Length _tracksplines))
  (if (>= TrackSplineIndex _returnvalue)
    ;[1 1 1] Print info about what went wrong
    (Development|PrintString (Utilities|String|Append "Bogie asked to change to track: " (Utilities|GetDisplayName Track) " but spline index: " (Utilities|String|ToString(Integer) TrackSplineIndex) " is out of bounds: " (Utilities|String|ToString(Integer) _returnvalue)))
    (else
      ;[1 1 1] Set the track, spline index and spline component
      (bind _output_get (Variables|BogieSettings|SetTrack Track))
      (bind _output_get_2 (Variables|BogieSettings|SetSplineIndex TrackSplineIndex))
      (bind _output_get_3 (Variables|Default|SetSplineComponent (Utilities|Struct|BreakS_TrackSpline (Utilities|Array|Get(acopy) (Variables|/Game/TrainAndRail/Blueprints/BP_TrainTrack.BP_TrainTrack_C|GetTrackSplines _output_get) _output_get_2))))
      ;[1 1 1] Set the distance on the track, doing a check to make sure it's a valid distance
      (bind _output_get_4 (Variables|BogieSettings|SetSplineLength (Spline|GetSplineLength _output_get_3)))
      (if (> DistanceOnTrack _output_get_4)
        (Variables|BogieSettings|SetSplineDistance _output_get_4)
        (else
          (Variables|BogieSettings|SetSplineDistance DistanceOnTrack)))
      (Variables|BogieSettings|SetNeedsAlignment false))))

(fn TickMovement
  (params (Speed :type Float%20%28single-precision%29%20%28by%20ref%29) (UpdateID :type Integer))
  (Variables|Default|SetUpdateID UpdateID)
  (Variables|BogieSettings|SetPreviousSplineDistance (Variables|BogieSettings|GetSplineDistance))
  ;[1 1 1] Increase our distance on the spline, if the direction of travel is inverted, subtract the increase
  (Variables|BogieSettings|SetSplineDistance (+ (Variables|BogieSettings|GetSplineDistance) (Math|Float|SelectFloat (* Speed -1.0) Speed (Variables|BogieSettings|GetInvertDirOfTravel)))))

(fn GetTransform
  (bind _splinecomponent (Variables|Default|GetSplineComponent))
  (bind _splinedistance (Variables|BogieSettings|GetSplineDistance))
  (bind _returnvalue (Spline|GetTransformatDistanceAlongSpline _splinecomponent _splinedistance "World" false))
  (bind (_location _rotation _scale) (Math|Transform|BreakTransform _returnvalue))
  (if (Variables|BogieSettings|GetInvertDirOfTravel)
    (return (Math|Transform|MakeTransform _location (Math|Rotator|CombineRotators (Math|Rotator|MakeRotator 0.0 0.0 1.8e+02) _rotation) _scale))
    (else
      ;[1 1 1] If the dir of travel isn't inverted, return the normal transform
      (return (Spline|GetTransformatDistanceAlongSpline (Variables|Default|GetSplineComponent) (Variables|BogieSettings|GetSplineDistance) "World" false)))))

(fn GetDistancetoEndOfTrack
  (params (Speed :type Float%20%28single-precision%29%20%28by%20ref%29))
  ;[1 1 1] If the speed is negative
  (if (< Speed 0.0)
    ;[1 1 1] If the direction of travel is inverted
    (if (Variables|BogieSettings|GetInvertDirOfTravel)
      (return (- (Variables|BogieSettings|GetSplineLength) (Variables|BogieSettings|GetSplineDistance)) true)
      (else
        (return (Variables|BogieSettings|GetSplineDistance) false)))
    (elif (Variables|BogieSettings|GetInvertDirOfTravel)
      (return (Variables|BogieSettings|GetSplineDistance) false)
      (else
        (return (- (Variables|BogieSettings|GetSplineLength) (Variables|BogieSettings|GetSplineDistance)) true)))))

(fn GetConnectionPoint
  (params (GetEndPoint :type Boolean%20%28by%20ref%29))
  (bind _track (Variables|BogieSettings|GetTrack))
  (bind _splineindex (Variables|BogieSettings|GetSplineIndex))
  (bind _tracksplines (Variables|/Game/TrainAndRail/Blueprints/BP_TrainTrack.BP_TrainTrack_C|GetTrackSplines _track))
  (bind _output (Utilities|Array|Get(acopy) _tracksplines _splineindex))
  (bind (_startconnectionpoint _endconnectionpoint) (Utilities|Struct|BreakS_TrackSpline _output))
  ;[1 1 1] Return the connection point for the track spline the bogie is currently on
  (if GetEndPoint
    (return _endconnectionpoint true)
    (else
      (return _startconnectionpoint false))))

(fn UpdateDistanceforEndOfClosedLoop
  (params (Speed :type Float%20%28single-precision%29%20%28by%20ref%29))
  (Variables|BogieSettings|SetSplineDistance (- Speed (Variables|BogieSettings|GetDistanceToEndOfTrack))))

(fn RestorePreviousDistance
  (params (UpdateReverseID :type Integer))
  (if (== UpdateReverseID (Variables|Default|GetUpdateID))
    (Variables|BogieSettings|SetSplineDistance (Variables|BogieSettings|GetPreviousSplineDistance))))

(fn GetLocation
  (return (.Location (Math|Transform|BreakTransform (CallFunction|GetTransform)))))

(fn GetRotation
  (return (.Rotation (Math|Transform|BreakTransform (CallFunction|GetTransform)))))