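; Blueprint function library for the train and rail system, providing track spline queries, validity checks and the tags for ignored or auto-added components.
; Closest distance on a spline is approximated by finding the two nearest points and sampling between them.
; FindLocationOnTracks recursively walks a signed distance across connected tracks, flipping direction at reversed connections.
; It records every traversed span and reports whether the requested distance was reached.
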(fn GetTrackIgnoreTag
  ;[1 1 1] Any spline component with this tag will not be used as a train track spline
  (return "ChooChooIgnore"))

(fn GetUsableSplinesfromTrack
  (params (SourceTrack :type BP%20Train%20Track%20Object%20Reference))
  ;[1 1 1] Get all spline components from a track that don't have the internal ignore tag
  (for _array_element (Actor|GetComponentsByClass SourceTrack "/Script/Engine.SplineComponent")
    (if (not (Components|ComponentHasTag _array_element (CallFunction|GetTrackIgnoreTag)))
      (Utilities|Array|Add (LocalVariables|GetUsableComponents) _array_element)))
  (return (LocalVariables|GetUsableComponents)))

(fn GetStartandEndLocationOfSpline
  (params (SplineComp :type Spline%20Component%20Object%20Reference))
  ;[1 1 1] Get the start and end world location of a spline
  (return (Spline|GetLocationatSplinePoint SplineComp 0 "World") (Spline|GetLocationatSplinePoint SplineComp (- (Spline|GetNumberOfSplinePoints SplineComp) 1) "World")))

(fn GetDistanceBetweenLocations
  (params (PointA :type Vector) (PointB :type Vector))
  ;[1 1 1] Find the distance between two locations
  (return (Math|Vector|VectorLength (- PointA PointB))))

(fn IsValidTrackSplineIndex
  (params (Track :type BP%20Train%20Track%20Object%20Reference) (SplineIndex :type Integer%20%28by%20ref%29))
  ;[1 1 1] Returns a bool indicating if the supplied index is a valid track spline index
  (return (< SplineIndex (Utilities|Array|Length (Variables|/Game/TrainAndRail/Blueprints/BP_TrainTrack.BP_TrainTrack_C|GetTrackSplines Track)))))

(fn HasTrackSplines
  (params (Track :type BP%20Train%20Track%20Object%20Reference))
  ;[1 1 1] Returns a bool indicating if this track has any track splines
  (return (> (Utilities|Array|Length (Variables|/Game/TrainAndRail/Blueprints/BP_TrainTrack.BP_TrainTrack_C|GetTrackSplines Track)) 0)))

(fn GetClosestSplinePoint
  (params (Spline :type Spline%20Component%20Object%20Reference%20%28by%20ref%29) (IgnorePoints :type Array%20of%20Integers) (Location :type Vector%20%28by%20ref%29))
  (bind _returnvalue (Spline|GetNumberOfSplinePoints Spline))
  (if (>= _returnvalue 2)
    ;[1 1 1] Loop through the spline points, ignore any on the ignore list
    (for _index (range 0 _returnvalue)
      (if (not (Utilities|Array|ContainsItem IgnorePoints _index)) ; If we are ignoring this point, skip it
        ;[1 1 1] Get the distance between the spline point and the supplied location, if it's lower than what we have, keep this point as the lowest and keep checking
        (if (< (CallFunction|GetDistanceBetweenLocations Location (Spline|GetLocationatSplinePoint Spline _index "World")) (LocalVariables|GetDistanceToPoint))
          (LocalVariables|SetDistanceToPoint (CallFunction|GetDistanceBetweenLocations Location (Spline|GetLocationatSplinePoint Spline _index "World")))
          (LocalVariables|SetReturnIndex _index))))
    (else
      ;[1 1 1] Send back the lowest point, -1 by default
      (Development|PrintString 0 "Not enough spline points on track, can't get closest location")))
  (return (LocalVariables|GetReturnIndex)))

(fn GetClosestDistanceonSpline
  (params (Spline :type Spline%20Component%20Object%20Reference%20%28by%20ref%29) (WorldLocation :type Vector%20%28by%20ref%29) (DistanceSampleCount :type Integer%20%28by%20ref%29))
  ;[1 1 1] First get the closest two spline points to the location
  (bind _closestpointindex (CallFunction|GetClosestSplinePoint Spline (Utilities|Array|MakeArray -1) WorldLocation))
  (bind _output_get (LocalVariables|SetPointA _closestpointindex))
  (bind _closestpointindex_2 (CallFunction|GetClosestSplinePoint Spline (Utilities|Array|MakeArray _output_get) WorldLocation))
  (LocalVariables|SetPointB _closestpointindex_2)
  ;[1 1 1] Make sure both points are valid
  (if (and (!= (LocalVariables|GetPointA) -1) (!= (LocalVariables|GetPointB) -1))
    ;[1 1 1] Get the closest location between the two points
    (bind _closestdistance (CallFunction|GetClosestDistanceBetweenSplinePoints Spline (LocalVariables|GetPointA) (LocalVariables|GetPointB) WorldLocation DistanceSampleCount))
    (LocalVariables|SetLowestDistance _closestdistance)
    (LocalVariables|SetValidReturn true)
    (else
      (Development|PrintString 0 (Utilities|String|Append "Failed to get closest disacne on spline, one or more points came back invalid. PointA: " (Utilities|String|ToString(Integer) (LocalVariables|GetPointA)) " PointB: " (Utilities|String|ToString(Integer) (LocalVariables|GetPointB))) true true "(R=0.870000,G=0.000000,B=0.000000,A=1.000000)" 5.0)))
  (return (LocalVariables|GetLowestDistance) (LocalVariables|GetValidReturn)))

(fn GetClosestDistanceBetweenSplinePoints
  (params (Spline :type Spline%20Component%20Object%20Reference) (PointA :type Integer%20%28by%20ref%29) (PointB :type Integer%20%28by%20ref%29) (WorldLocation :type Vector%20%28by%20ref%29) (NumDistanceSamples :type Integer))
  ;[1 1 1] First pick the lowest point as the start point, highest point as the end point
  (bind _output_get (LocalVariables|SetEndPoint (Math|Integer|SelectInt PointA PointB (> PointA PointB))))
  (LocalVariables|SetStartPoint (Math|Integer|SelectInt PointA PointB (== _output_get PointB)))
  ;[1 1 1] Grab the distance from our start and end
  (LocalVariables|SetStartDistance (Spline|GetDistanceAlongSplineatSplinePoint Spline (LocalVariables|GetStartPoint)))
  (LocalVariables|SetEndDistance (Spline|GetDistanceAlongSplineatSplinePoint Spline (LocalVariables|GetEndPoint)))
  ;[1 1 1] Setup our distance sample and current distance on the spline
  (LocalVariables|SetDistanceSample (/ (- (LocalVariables|GetEndDistance) (LocalVariables|GetStartDistance)) (Math|Conversions|ToFloat(Integer) NumDistanceSamples)))
  (LocalVariables|SetCurrentSampleDistance (LocalVariables|GetStartDistance))
  (for _index (range 0 NumDistanceSamples)
    ;[1 1 1] Get the location at the distance and check it against our closest distance, update and keep checking until we hit the end
    (bind _output_get_2 (LocalVariables|SetCurrentSampleDistance (+ (* _index (LocalVariables|GetDistanceSample)) (LocalVariables|GetStartDistance))))
    (if (<= (CallFunction|GetDistanceBetweenLocations (Spline|GetLocationatDistanceAlongSpline Spline _output_get_2 "World") WorldLocation) (LocalVariables|GetDistanceToClosestPoint))
      (LocalVariables|SetDistanceToClosestPoint (CallFunction|GetDistanceBetweenLocations (Spline|GetLocationatDistanceAlongSpline Spline _output_get_2 "World") WorldLocation))
      (LocalVariables|SetReturnDistance (LocalVariables|GetCurrentSampleDistance))))
  (return (LocalVariables|GetReturnDistance)))

(fn FindLocationonTracks
  (params (StartingTrack :type BP%20Train%20Track%20Object%20Reference) (StartingTrackSpline :type S%20Track%20Spline%20Structure%20%28by%20ref%29) (StartingDistance :type Float%20%28single-precision%29%20%28by%20ref%29) (RequestedDistance :type Float%20%28single-precision%29%20%28by%20ref%29) (Invert :type Boolean) (CurrentPassThroughInfo :type Array%20of%20S%20Track%20Pass%20Through%20Info%20Structures))
  ;[1 1 1] Setup some handy variables to keep things cleaner
  (LocalVariables|SetUpdatedPassThroughInfo CurrentPassThroughInfo)
  (LocalVariables|SetPassedInDoInvert Invert)
  (LocalVariables|SetStartTrack StartingTrack)
  (LocalVariables|SetStartTrackSpline StartingTrackSpline)
  (LocalVariables|SetStartDistance StartingDistance)
  (LocalVariables|SetReqDistance (Math|Float|SelectFloat (* RequestedDistance -1.0) RequestedDistance (LocalVariables|GetPassedInDoInvert)))
  ;[1 1 1] Set the spline length
  (LocalVariables|SetStartTrackSplineLength (Spline|GetSplineLength (Utilities|Struct|BreakS_TrackSpline (LocalVariables|GetStartTrackSpline))))
  ;[1 1 1] If distance is +, then it's going forward down the tracks
  (if (< (LocalVariables|GetReqDistance) 0.0)
    (if (>= (LocalVariables|GetStartDistance) (Math|Float|Absolute(Float) (LocalVariables|GetReqDistance)))
      (Utilities|Array|Add (LocalVariables|GetUpdatedPassThroughInfo) (Utilities|Struct|MakeS_TrackPassThroughInfo (LocalVariables|GetStartTrack) (LocalVariables|GetStartTrackSpline) (.Lowest (CallFunction|GetLowestFloat (LocalVariables|GetStartDistance) (+ (LocalVariables|GetStartDistance) (LocalVariables|GetReqDistance)))) (.Highest (CallFunction|GetLowestFloat (LocalVariables|GetStartDistance) (+ (LocalVariables|GetStartDistance) (LocalVariables|GetReqDistance)))) (LocalVariables|GetPassedInDoInvert)))
      ;[1 1 1] Send back the final location
      (return (LocalVariables|GetStartTrack) (LocalVariables|GetStartTrackSpline) (+ (LocalVariables|GetStartDistance) (LocalVariables|GetReqDistance)) true (LocalVariables|GetPassedInDoInvert) (LocalVariables|GetUpdatedPassThroughInfo))
      (else
        ;[1 1 1] Update the required distance with the distance traveled on this spline
        (Utilities|Array|Add (LocalVariables|GetUpdatedPassThroughInfo) (Utilities|Struct|MakeS_TrackPassThroughInfo (LocalVariables|GetStartTrack) (LocalVariables|GetStartTrackSpline) (.Lowest (CallFunction|GetLowestFloat (LocalVariables|GetStartDistance) (Math|Float|Clamp(Float) (+ (LocalVariables|GetReqDistance) (LocalVariables|GetStartDistance)) 0.0 (LocalVariables|GetStartTrackSplineLength)))) (.Highest (CallFunction|GetLowestFloat (LocalVariables|GetStartDistance) (Math|Float|Clamp(Float) (+ (LocalVariables|GetReqDistance) (LocalVariables|GetStartDistance)) 0.0 (LocalVariables|GetStartTrackSplineLength)))) (LocalVariables|GetPassedInDoInvert)))
        (LocalVariables|SetReqDistance (+ (LocalVariables|GetReqDistance) (LocalVariables|GetStartDistance)))
        (bind (_connection _connectionfound) (Default|PickConnectiontoUse (LocalVariables|GetStartTrack) (Utilities|Struct|BreakS_TrackSpline (LocalVariables|GetStartTrackSpline)) false))
        (if _connectionfound
          ;[1 1 1] Here we are going backwards on a spline, so we expect the spline we are connecting into to be an end location, if it's not, we need to invert the required distance and adjust our starting location on the connecting spline
          (LocalVariables|SetDoInvert (Utilities|Enum|Equal(Enum) (.Location (Utilities|Struct|BreakS_TrackConnection _connection)) "NewEnumerator0"))
          (bind (_endtrack _endtrackspline _enddistance _endreached _inverteddiroftravel _travelinfo) (CallFunction|FindLocationonTracks (.Track (Utilities|Struct|BreakS_TrackConnection _connection)) (.TrackSpline (Default|GetTrackSplinebyIndex (.Track (Utilities|Struct|BreakS_TrackConnection _connection)) (.ConnectionID (Utilities|Struct|BreakS_TrackConnection _connection)))) (Math|Float|SelectFloat 0.0 (Spline|GetSplineLength (.Spline (Utilities|Struct|BreakS_TrackSpline (.TrackSpline (Default|GetTrackSplinebyIndex (.Track (Utilities|Struct|BreakS_TrackConnection _connection)) (.ConnectionID (Utilities|Struct|BreakS_TrackConnection _connection))))))) (LocalVariables|GetDoInvert)) (LocalVariables|GetReqDistance) (LocalVariables|GetDoInvert) (LocalVariables|GetUpdatedPassThroughInfo)))
          (return _endtrack _endtrackspline _enddistance _endreached _inverteddiroftravel _travelinfo)
          (else
            ;[1 1 1] Send back the error, but include all the info so it can be used
            (return (LocalVariables|GetStartTrack) (LocalVariables|GetStartTrackSpline) 0.0 false (LocalVariables|GetPassedInDoInvert) (LocalVariables|GetUpdatedPassThroughInfo))))))
    (elif (>= (LocalVariables|GetStartTrackSplineLength) (+ (LocalVariables|GetReqDistance) (LocalVariables|GetStartDistance)))
      (Utilities|Array|Add (LocalVariables|GetUpdatedPassThroughInfo) (Utilities|Struct|MakeS_TrackPassThroughInfo (LocalVariables|GetStartTrack) (LocalVariables|GetStartTrackSpline) (.Lowest (CallFunction|GetLowestFloat (LocalVariables|GetStartDistance) (+ (LocalVariables|GetReqDistance) (LocalVariables|GetStartDistance)))) (.Highest (CallFunction|GetLowestFloat (LocalVariables|GetStartDistance) (+ (LocalVariables|GetReqDistance) (LocalVariables|GetStartDistance)))) (LocalVariables|GetPassedInDoInvert)))
      ;[1 1 1] Send back the final location
      (return (LocalVariables|GetStartTrack) (LocalVariables|GetStartTrackSpline) (+ (LocalVariables|GetReqDistance) (LocalVariables|GetStartDistance)) true (LocalVariables|GetPassedInDoInvert) (LocalVariables|GetUpdatedPassThroughInfo))
      (else
        ;[1 1 1] Update the required distance with the distance used on this spline
        (Utilities|Array|Add (LocalVariables|GetUpdatedPassThroughInfo) (Utilities|Struct|MakeS_TrackPassThroughInfo (LocalVariables|GetStartTrack) (LocalVariables|GetStartTrackSpline) (.Lowest (CallFunction|GetLowestFloat (LocalVariables|GetStartDistance) (+ (LocalVariables|GetStartDistance) (- (LocalVariables|GetStartTrackSplineLength) (LocalVariables|GetStartDistance))))) (.Highest (CallFunction|GetLowestFloat (LocalVariables|GetStartDistance) (+ (LocalVariables|GetStartDistance) (- (LocalVariables|GetStartTrackSplineLength) (LocalVariables|GetStartDistance))))) (LocalVariables|GetPassedInDoInvert)))
        (LocalVariables|SetReqDistance (- (LocalVariables|GetReqDistance) (- (LocalVariables|GetStartTrackSplineLength) (LocalVariables|GetStartDistance))))
        (bind (_connection_2 _connectionfound_2) (Default|PickConnectiontoUse (LocalVariables|GetStartTrack) (Utilities|Struct|BreakS_TrackSpline (LocalVariables|GetStartTrackSpline)) false))
        (if _connectionfound_2
          ;[1 1 1] Here we are going forward on the spline, so we expect to connect into the start location of the next track spline, if it's not and it's an end connection,we need to invert our required distance and adjust our starting location
          (LocalVariables|SetDoInvert (Utilities|Enum|Equal(Enum) (.Location (Utilities|Struct|BreakS_TrackConnection _connection_2)) "NewEnumerator1"))
          (bind (_endtrack_2 _endtrackspline_2 _enddistance_2 _endreached_2 _inverteddiroftravel_2 _travelinfo_2) (CallFunction|FindLocationonTracks (.Track (Utilities|Struct|BreakS_TrackConnection _connection_2)) (.TrackSpline (Default|GetTrackSplinebyIndex (.Track (Utilities|Struct|BreakS_TrackConnection _connection_2)) (.ConnectionID (Utilities|Struct|BreakS_TrackConnection _connection_2)))) (Math|Float|SelectFloat (Spline|GetSplineLength (Utilities|Struct|BreakS_TrackSpline (.TrackSpline (Default|GetTrackSplinebyIndex (.Track (Utilities|Struct|BreakS_TrackConnection _connection_2)) (.ConnectionID (Utilities|Struct|BreakS_TrackConnection _connection_2)))))) 0.0 (LocalVariables|GetDoInvert)) (LocalVariables|GetReqDistance) (LocalVariables|GetDoInvert) (LocalVariables|GetUpdatedPassThroughInfo)))
          (return _endtrack_2 _endtrackspline_2 _enddistance_2 _endreached_2 _inverteddiroftravel_2 _travelinfo_2)
          (else
            ;[1 1 1] Send back the error, but include all the info so it can be used
            (return (LocalVariables|GetStartTrack) (LocalVariables|GetStartTrackSpline) (LocalVariables|GetStartTrackSplineLength) false (LocalVariables|GetPassedInDoInvert) (LocalVariables|GetUpdatedPassThroughInfo))))))))

(fn GetLowestFloat
  (params (ValueA :type Float%20%28single-precision%29%20%28by%20ref%29) (ValueB :type Float%20%28single-precision%29%20%28by%20ref%29))
  ;[1 1 1] Return the lowest float from two passed in
  (return (Math|Float|SelectFloat ValueA ValueB (<= ValueA ValueB)) (Math|Float|SelectFloat ValueA ValueB (>= ValueA ValueB))))

(fn GetInternalCompTag
  ;[0.2395 1 0.9901] Used when auto creating components, such as arrows for tracks. So we know we can delete without issue later
  (return "ChooChooAutoAdded"))