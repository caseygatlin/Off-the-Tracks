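; Debug actor for the train and rail system, driven by boolean toggles and lists of selected tracks and carriages.
; Its construction script rebuilds track connections, prints connection info, marks trigger regions with box components and refreshes demo info boxes.
; Tick draws debug shapes for selected carriages' hitches, bogies and sensor boxes, plus bogie name labels.
; A function to clear all trigger regions exists but is not called here.
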(event EventBeginPlay)

(event Collision|EventActorBeginOverlap
  (params (OtherActor :type Actor%20Object%20Reference)))

(event EventTick
  (params (DeltaSeconds :type Float%20%28single-precision%29))
  (CallFunction|SelCarDisplaySensorBogie)
  (CallFunction|SelCarPrintAllBogieNames)
  (CallFunction|SelCarShowDebugHitch))

(fn ConstructionScript
  (CallFunction|ConnRebuildAllConnections)
  (CallFunction|ConnPrintConnectionInfoforAllTracks)
  (CallFunction|ConnPrintConnInfoforSelectedTrack)
  (CallFunction|TrackPrintTriggerRegions)
  (CallFunction|DemoRefreshInfoBoxes))

(fn ConnRebuildAllConnections
  ;[1 1 1] Force all tracks to rebuild their connections
  (if (Variables|ConnectionDebug|GetRebuildAllConnections)
    (Development|PrintString "-- Forcing all tracks to rebuild connections --")
    (bind _outactors (Actor|GetAllActorsOfClass "/Game/TrainAndRail/Blueprints/BP_TrainTrack.BP_TrainTrack_C"))
    (for _array_element _outactors
      (Default|RebuildTrackConnections _array_element))
    (Development|PrintString "-- Forced Connection Rebuild Complete --")))

(fn ConnPrintConnectionInfoforAllTracks
  (if (Variables|ConnectionDebug|GetPrintConnInfoForAllTracks)
    (bind _outactors (Actor|GetAllActorsOfClass "/Game/TrainAndRail/Blueprints/BP_TrainTrack.BP_TrainTrack_C"))
    (for _array_element _outactors
      (CallFunction|PrintConnectionInfoforTrack _array_element))))

(fn PrintConnectionInfoforTrack
  (params (Track :type BP%20Train%20Track%20Object%20Reference))
  (bind _tracksplines (Variables|/Game/TrainAndRail/Blueprints/BP_TrainTrack.BP_TrainTrack_C|GetTrackSplines Track))
  (Development|PrintString (Utilities|String|Append "--- Track: " (Utilities|GetDisplayName Track) " has " (Utilities|String|ToString(Integer) (Utilities|Array|Length _tracksplines)) " track splines ---"))
  (for _array_element _tracksplines
    (CallFunction|PrintConnectionPointInfo (.StartConnectionPoint (Utilities|Struct|BreakS_TrackSpline _array_element)) "Starting Connection Point")
    (CallFunction|PrintConnectionPointInfo (.EndConnectionPoint (Utilities|Struct|BreakS_TrackSpline _array_element)) "Ending Connection Point")))

(fn ConnPrintConnInfoforSelectedTrack
  (if (Variables|ConnectionDebug|GetPrintConnInfoForSelectedTrack)
    (for _array_element (Variables|Selected|GetSelectedTracks)
      (CallFunction|PrintConnectionInfoforTrack _array_element))))

(fn PrintConnectionPointInfo
  (params (ConnectionPoint :type S%20Track%20Connection%20Point%20Structure) (Name :type String))
  (bind _connections (Utilities|Struct|BreakS_TrackConnectionPoint ConnectionPoint))
  (Development|PrintString (Utilities|String|Append Name " - " (Utilities|String|ToString(Integer) (Utilities|Array|Length _connections)) " connections"))
  (for _array_element _connections
    (Development|PrintString (Utilities|String|Append "    Conn: " (Utilities|String|ToString(Integer) (.ConnectionID (Utilities|Struct|BreakS_TrackConnection _array_element))) " Location: " (Utilities|String|EnumtoString (.Location (Utilities|Struct|BreakS_TrackConnection _array_element))) " Track: " (Utilities|GetDisplayName (.Track (Utilities|Struct|BreakS_TrackConnection _array_element)))))))

(fn SelCarPrintAllBogieNames
  (if (Variables|Carriage|GetSelCar_PrintBogieNames)
    (for _array_element (Variables|Selected|GetSelectedCarriages)
      (Utilities|IsValid _array_element
        (:Is%20Valid
          (for _array_element_2 (Variables|/Game/TrainAndRail/Blueprints/BP_TrainCarriage.BP_TrainCarriage_C|GetBogies _array_element)
            (Rendering|Debug|DrawDebugString (.Location (Math|Transform|BreakTransform (Default|GetTransform _array_element_2))) (Variables|/Game/TrainAndRail/Blueprints/AC_Bogie.AC_Bogie_C|GetDebugName _array_element_2) 0 "(R=0.025297,G=0.000000,B=1.000000,A=1.000000)" 0.004)
            (Rendering|Debug|DrawDebugSphere (.Location (Math|Transform|BreakTransform (Default|GetTransform _array_element_2))) 5e+01 8 "(R=0.000000,G=0.481161,B=1.000000,A=1.000000)" 0.05 1.0)))))))

(fn TrackPrintTriggerRegions
  (if (Variables|Tracks|GetPrintTriggerRegions)
    (for _array_element (Variables|Selected|GetSelectedTracks)
      (Development|PrintString (Utilities|String|Append "\\\\\\ Track " (Utilities|GetDisplayName _array_element) " has " (Utilities|String|ToString(Integer) (Utilities|Array|Length (Variables|/Game/TrainAndRail/Blueprints/BP_TrainTrack.BP_TrainTrack_C|GetTriggerRegions _array_element))) " trigger regions ///"))
      ;[1 1 1] Loop through each of the regions and add a col box as a rough marker for the region
      (for (_array_element_2 _array_index) (Variables|/Game/TrainAndRail/Blueprints/BP_TrainTrack.BP_TrainTrack_C|GetTriggerRegions _array_element)
        (Development|PrintString (Utilities|String|Append "     TR " (Utilities|String|ToString(Integer) _array_index) " " (Utilities|GetDisplayName (.Trigger (Utilities|Struct|BreakS_TrackTriggerRegion _array_element_2))) " Start: " (Utilities|String|ToString(Float) (.StartDistance (Utilities|Struct|BreakS_TrackRegion (.Region (Utilities|Struct|BreakS_TrackTriggerRegion _array_element_2))))) " End: " (Utilities|String|ToString(Float) (.EndDistance (Utilities|Struct|BreakS_TrackRegion (.Region (Utilities|Struct|BreakS_TrackTriggerRegion _array_element_2))))) " on spline: " (Utilities|GetDisplayName (.Spline (Utilities|Struct|BreakS_TrackSpline (.TrackSpline (Default|GetTrackSplinebyIndex _array_element (.TrackSplineIndex (Utilities|Struct|BreakS_TrackRegion (.Region (Utilities|Struct|BreakS_TrackTriggerRegion _array_element_2)))))))))))
        (LocalVariables|SetStarDist (.StartDistance (Utilities|Struct|BreakS_TrackRegion (.Region (Utilities|Struct|BreakS_TrackTriggerRegion _array_element_2)))))
        (LocalVariables|SetEndDist (.EndDistance (Utilities|Struct|BreakS_TrackRegion (.Region (Utilities|Struct|BreakS_TrackTriggerRegion _array_element_2)))))
        (LocalVariables|SetStartVec (Spline|GetLocationatDistanceAlongSpline (.Spline (Utilities|Struct|BreakS_TrackSpline (.TrackSpline (Default|GetTrackSplinebyIndex _array_element (.TrackSplineIndex (Utilities|Struct|BreakS_TrackRegion (.Region (Utilities|Struct|BreakS_TrackTriggerRegion _array_element_2)))))))) (.StartDistance (Utilities|Struct|BreakS_TrackRegion (.Region (Utilities|Struct|BreakS_TrackTriggerRegion _array_element_2)))) "World"))
        (LocalVariables|SetEndVec (Spline|GetLocationatDistanceAlongSpline (.Spline (Utilities|Struct|BreakS_TrackSpline (.TrackSpline (Default|GetTrackSplinebyIndex _array_element (.TrackSplineIndex (Utilities|Struct|BreakS_TrackRegion (.Region (Utilities|Struct|BreakS_TrackTriggerRegion _array_element_2)))))))) (.EndDistance (Utilities|Struct|BreakS_TrackRegion (.Region (Utilities|Struct|BreakS_TrackTriggerRegion _array_element_2)))) "World"))
        (bind _returnvalue (AddComponent|AddBoxComponent true))
        (Components|Box|SetBoxExtent _returnvalue (Math|Vector|MakeVector (/ (- (LocalVariables|GetStarDist) (LocalVariables|GetEndDist)) 2.0) 1e+02 1e+02) true)
        (Collision|SetCollisionEnabled _returnvalue "NoCollision")
        (Development|SetHiddeninGame _returnvalue false false)
        (Transformation|SetWorldTransform _returnvalue (Math|Transform|MakeTransform (/ (+ (LocalVariables|GetStartVec) (LocalVariables|GetEndVec)) 2.0) (Math|Rotator|FindLookatRotation (LocalVariables|GetStartVec) (LocalVariables|GetEndVec))) false true)))))

(fn TrackDeleteAllTriggerRegions
  (if (Variables|Tracks|GetDeleteAllTriggerRegions)
    (bind _outactors (Actor|GetAllActorsOfClass "/Game/TrainAndRail/Blueprints/BP_TrainTrack.BP_TrainTrack_C"))
    (for _array_element _outactors
      (Default|ClearTriggerRegions _array_element 0 true))))

(fn SelCarShowDebugHitch
  (bind _returnvalue (Math|Float|MakeLiteralFloat 0.02))
  (if (Variables|Carriage|GetSelCar_ShowDebugHitches)
    (for _array_element (Variables|Selected|GetSelectedCarriages)
      (Rendering|Debug|DrawDebugSphere (Transformation|GetWorldLocation (Variables|/Game/TrainAndRail/Blueprints/BP_TrainCarriage.BP_TrainCarriage_C|GetFrontHitch _array_element)) (Variables|/Script/Engine.SphereComponent|GetSphereRadius (Variables|/Game/TrainAndRail/Blueprints/BP_TrainCarriage.BP_TrainCarriage_C|GetFrontHitch _array_element)) 12 "(R=0.029500,G=0.520000,B=0.033831,A=1.000000)" _returnvalue 2.0)
      (Rendering|Debug|DrawDebugSphere (Transformation|GetWorldLocation (Variables|/Game/TrainAndRail/Blueprints/BP_TrainCarriage.BP_TrainCarriage_C|GetRearHitch _array_element)) (Variables|/Script/Engine.SphereComponent|GetSphereRadius (Variables|/Game/TrainAndRail/Blueprints/BP_TrainCarriage.BP_TrainCarriage_C|GetRearHitch _array_element)) 12 "(R=0.495000,G=0.000000,B=0.088596,A=1.000000)" _returnvalue 2.0))))

(fn SelCarDisplaySensorBogie
  (if (Variables|Carriage|GetSelCar_ShowSensorBogie)
    (for _array_element (Variables|Selected|GetSelectedCarriages)
      (if (not (Variables|/Game/TrainAndRail/Blueprints/BP_TrainCarriage.BP_TrainCarriage_C|GetDisableSensorBogie _array_element))
        (LocalVariables|SetSensorOffset (Variables|/Game/TrainAndRail/Blueprints/BP_TrainCarriage.BP_TrainCarriage_C|GetSensorOffset _array_element))
        (LocalVariables|SetSensorBoxSize (Variables|/Game/TrainAndRail/Blueprints/BP_TrainCarriage.BP_TrainCarriage_C|GetSensorBoxSize _array_element))
        (Rendering|Debug|DrawDebugString (.Location (Math|Transform|BreakTransform (Default|GetTransform (Variables|/Game/TrainAndRail/Blueprints/BP_TrainCarriage.BP_TrainCarriage_C|GetSensorBogie _array_element)))) (Variables|/Game/TrainAndRail/Blueprints/AC_Bogie.AC_Bogie_C|GetDebugName (Variables|/Game/TrainAndRail/Blueprints/BP_TrainCarriage.BP_TrainCarriage_C|GetSensorBogie _array_element)) 0 "(R=0.129725,G=1.000000,B=0.305074,A=1.000000)" (Variables|RenderSettings|GetDebugTextTimeOnScreen))
        (Rendering|Debug|DrawDebugSphere (.Location (Math|Transform|BreakTransform (Default|GetTransform (Variables|/Game/TrainAndRail/Blueprints/BP_TrainCarriage.BP_TrainCarriage_C|GetSensorBogie _array_element)))) 5e+01 8 "(R=0.000000,G=0.481161,B=1.000000,A=1.000000)" (Variables|RenderSettings|GetDebugShapeTimeOnScreen) 1.0)
        (Rendering|Debug|DrawDebugBox (+ (.Location (Math|Transform|BreakTransform (Default|GetTransform (Variables|/Game/TrainAndRail/Blueprints/BP_TrainCarriage.BP_TrainCarriage_C|GetSensorBogie _array_element)))) (Math|Vector|RotateVector (LocalVariables|GetSensorOffset) (.Rotation (Math|Transform|BreakTransform (Default|GetTransform (Variables|/Game/TrainAndRail/Blueprints/BP_TrainCarriage.BP_TrainCarriage_C|GetSensorBogie _array_element)))))) (LocalVariables|GetSensorBoxSize) "(R=0.000000,G=0.187191,B=1.000000,A=1.000000)" (.Rotation (Math|Transform|BreakTransform (Default|GetTransform (Variables|/Game/TrainAndRail/Blueprints/BP_TrainCarriage.BP_TrainCarriage_C|GetSensorBogie _array_element)))) (Variables|RenderSettings|GetDebugShapeTimeOnScreen) 0.0)))))

(fn DemoRefreshInfoBoxes
  (if (Variables|Demo|GetRefreshDemoInfoBoxes)
    (Utilities|FlowControl|Sequence
      (:then_0
        (bind _outactors (Actor|GetAllActorsOfClass "/Game/TrainAndRail/DemoHellpers/Demo_InfoBox_Footer.Demo_InfoBox_Footer_C"))
        (for _array_element _outactors
          (Default|RefreshInfo _array_element)))
      (:then_1
        (bind _outactors_2 (Actor|GetAllActorsOfClass "/Game/TrainAndRail/DemoHellpers/Demo_InfoBox_Tall.Demo_InfoBox_Tall_C"))
        (for _array_element_2 _outactors_2
          (Default|RefreshInfo _array_element_2))))))