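; CameraFollowActor is a main menu actor that smoothly follows a Target actor's location and rotation, by its name to carry the camera.
; It snaps to the Target's transform on BeginPlay.
; Each Tick it lerps toward the Target using delta time times Speed as alpha, giving an eased follow with shortest-path rotation.
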(event EventBeginPlay
  (Transformation|SetActorLocationAndRotation (Transformation|GetActorLocation (Variables|Default|GetTarget)) (Transformation|GetActorRotation (Variables|Default|GetTarget))))

(event EventTick
  (params (DeltaSeconds :type Float%20%28single-precision%29))
  (bind _speed (Variables|Default|GetSpeed))
  (bind _returnvalue (* DeltaSeconds _speed))
  (Transformation|SetActorLocationAndRotation (Math|Vector|Lerp(Vector) (Transformation|GetActorLocation) (Transformation|GetActorLocation (Variables|Default|GetTarget)) _returnvalue) (Math|Rotator|Lerp(Rotator) (Transformation|GetActorRotation) (Transformation|GetActorRotation (Variables|Default|GetTarget)) _returnvalue true)))

(fn ConstructionScript)