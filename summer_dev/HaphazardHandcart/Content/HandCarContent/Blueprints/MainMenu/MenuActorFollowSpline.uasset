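; Main menu actor that travels along the spline path of a referenced track.
; When Active, BeginPlay starts Move, which runs a timeline at a rate of 1/Duration from StartOffset.
; Each update maps the timeline alpha to distance along the spline and sets the actor's location in world space and rotation from the spline's local-space rotation.
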(event Custom|Move
  (Components|Timeline|SetPlayRate (Variables|Default|GetSplineMover) (/ 1.0 (Variables|Default|Getduration)))
  (Components|Timeline|SetNewTime (Variables|Default|GetSplineMover) (Variables|Default|GetStartOffset))
  (bind _alpha (Timeline|SplineMover Play)
    (:Update
      (Variables|Default|SetAlpha _alpha)
      (Transformation|SetActorLocationAndRotation (Spline|GetLocationatDistanceAlongSpline (Variables|/Game/HandCarContent/Blueprints/MainMenu/CameraTrack.CameraTrack_C|GetSplinePath (Variables|Default|GetTrackRef)) (Math|Float|Lerp 0.0 (Spline|GetSplineLength (Variables|/Game/HandCarContent/Blueprints/MainMenu/CameraTrack.CameraTrack_C|GetSplinePath (Variables|Default|GetTrackRef))) (Variables|Default|GetAlpha)) "World") (Spline|GetRotationatDistanceAlongSpline (Variables|/Game/HandCarContent/Blueprints/MainMenu/CameraTrack.CameraTrack_C|GetSplinePath (Variables|Default|GetTrackRef)) (Math|Float|Lerp 0.0 (Spline|GetSplineLength (Variables|/Game/HandCarContent/Blueprints/MainMenu/CameraTrack.CameraTrack_C|GetSplinePath (Variables|Default|GetTrackRef))) (Variables|Default|GetAlpha)) "Local")))))

(event EventBeginPlay
  (if (Variables|Default|GetActive)
    (CallFunction|Move)))

(fn ConstructionScript)