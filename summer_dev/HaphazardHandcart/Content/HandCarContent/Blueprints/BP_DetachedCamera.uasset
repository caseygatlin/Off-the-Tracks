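; BP_DetachedCamera is the camera for the player handcar, adding a zoom effect while the cart boosts.
; BeginPlay caches the default horizontal offset and field of view, then casts MPlayerHandcar to BP_PlayerHandcar.
; Each Tick, UpdateZoomEffects reads the boost state and picks either those defaults or defaults plus boost offsets as targets.
; Constant-speed interpolation moves camera distance (MHorizontalOffset) and FOV toward them, each at its own rate.
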(event EventBeginPlay
  (Variables|BoostEffect|SetCameraDistanceDefault (Variables|Default|Getm_HorizontalOffset))
  (Variables|BoostEffect|SetCameraFovDefault (Variables|/Script/Engine.CameraComponent|GetFieldOfView (Variables|Default|Getm_Camera)))
  (bind _asbp_player_handcar (Utilities|Casting|CastToBP_PlayerHandcar (Variables|Default|Getm_PlayerHandcar)))
  (Variables|Default|Setplayer _asbp_player_handcar))

(event Collision|EventActorBeginOverlap
  (params (OtherActor :type Actor%20Object%20Reference)))

(event EventTick
  (params (DeltaSeconds :type Float%20%28single-precision%29))
  (CallFunction|UpdateZoomEffects DeltaSeconds))

(fn ConstructionScript)

(fn UpdateZoomEffects
  (params (DeletaTime :type Float%20%28single-precision%29))
  (LocalVariables|SetDeltaTime DeletaTime)
  (if (Class|PlayerHandcar|GetCartBoostState (Variables|Default|Getplayer))
    (LocalVariables|SetFOVLocalTarget (+ (Variables|BoostEffect|GetCameraFovDefault) (Variables|BoostEffect|GetCameraBoostEffectFOVTargetOffset)))
    (LocalVariables|SetDistanceLocalTarget (+ (Variables|BoostEffect|GetCameraDistanceDefault) (Variables|BoostEffect|GetCameraBoostEffectDistanceTargetOffset)))
    (else
      (LocalVariables|SetFOVLocalTarget (Variables|BoostEffect|GetCameraFovDefault))
      (LocalVariables|SetDistanceLocalTarget (Variables|BoostEffect|GetCameraDistanceDefault))))
  (Variables|Default|Setm_HorizontalOffset (Math|Interpolation|FInterptoConstant (Variables|Default|Getm_HorizontalOffset) (LocalVariables|GetDistanceLocalTarget) (LocalVariables|GetDeltaTime) (Variables|BoostEffect|GetDistanceLerpSpeed)))
  (Camera|SetFieldOfView (Variables|Default|Getm_Camera) (Math|Interpolation|FInterptoConstant (Variables|/Script/Engine.CameraComponent|GetFieldOfView (Variables|Default|Getm_Camera)) (LocalVariables|GetFOVLocalTarget) (LocalVariables|GetDeltaTime) (Variables|BoostEffect|GetFOVLerpSpeed))))