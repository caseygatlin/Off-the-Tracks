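; Player-driven mine cart, a train carriage that rides rails by pumping a handle and can jump between tracks.
; Smoothed gyro or W/E input rotates the handle; pump strokes set a boost timer that releases the brakes, with mass adjusted on slopes.
; Jumps detach the cart and launch it with physics, biased by lean input, until overlapping a BP_TrainTrack reattaches it.
; Tilt toggles sparks; lean-state, obstacle and jump-tick functions are empty.
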(event Custom|WKeyPressed
  (if (not (Variables|JumpSettings|GetIsJumping))
    (if (Variables|Default|GetIsRightHandleDown)
      (Variables|Default|SetIsRightHandleDown false)
      (CallFunction|ProcessInput 0.2)
      (if (Utilities|Enum|NotEqual(Enum) (Variables|Default|GetCarriageState) "NewEnumerator2")
        (CallFunction|ApplyPump 1.0)))))

(event Custom|EKeyPressed
  (if (not (Variables|JumpSettings|GetIsJumping))
    (if (not (Variables|Default|GetIsRightHandleDown))
      (Variables|Default|SetIsRightHandleDown true)
      (CallFunction|ProcessInput 0.8)
      (if (Utilities|Enum|NotEqual(Enum) (Variables|Default|GetCarriageState) "NewEnumerator2")
        (CallFunction|ApplyPump 1.0)))))

(event EventBeginPlay
  (|CallParentFunction)
  (Variables|Default|SetSavedMass (Variables|Default|GetMass))
  (Utilities|Array|Add (Variables|DebugVariables|GetDebugOutArray) "Time,Lean,Pump"))

(event EventTick
  (params (DeltaSeconds :type Float%20%28single-precision%29))
  (bind _leanamountneeded (Variables|Default|GetLeanAmountNeeded))
  (bind _leanamountneeded_2 (Variables|Default|GetLeanAmountNeeded))
  (bind _returnvalue (* _leanamountneeded -1.0))
  (if (not (Variables|JumpSettings|GetIsJumping))
    (Utilities|FlowControl|Sequence
      (:then_0
        (|CallParentFunction DeltaSeconds)
        (if (Variables|PlayerLockout|GetPlayerControlLockout)
          (CallFunction|HandleNonPlayerControl)
          (else
            (CallFunction|HandleGyroInput)))
        (CallFunction|CheckLeanStateforSparks)
        (Variables|Default|SetTimeSinceLastPump (+ (Variables|Default|GetTimeSinceLastPump) DeltaSeconds))
        (if (Utilities|Enum|Equal(Enum) (Variables|Default|GetCarriageState) "NewEnumerator0")
          (CallFunction|ApplyorReleaseBrakes false)
          (CallFunction|SetCarriageState "NewEnumerator1" false)
          (Variables|Default|SetMass (Variables|Default|GetSavedMass)))
        ;[1 1 1] Tick the jump if we are jumping
        (if (Variables|JumpSettings|GetIsJumping)
          (CallFunction|TickJump DeltaSeconds))
        (if (Utilities|Enum|NotEqual(Enum) (Variables|Default|GetCarriageState) "NewEnumerator2")
          (if (> (Variables|Default|GetPumpTimer) 0.0)
            (Variables|Default|SetPumpTimer (- (Variables|Default|GetPumpTimer) DeltaSeconds))
            (CallFunction|UpdateDynamicMass)
            (CallFunction|ApplyorReleaseBrakes false)
            (CallFunction|SetCarriageState "NewEnumerator1" false)
            (else
              (CallFunction|ApplyorReleaseBrakes true)))))
      (:then_1
        (if (or (Variables|Default|GetDebug_LeanLeft) (Variables|Default|GetDebug_LeanRight))
          (if (Variables|Default|GetDebug_LeanLeft)
            (CallFunction|SetCartLeanState _returnvalue)
            (Variables|Default|SetCurrentLeanAmount _returnvalue)
            (elif (Variables|Default|GetDebug_LeanRight)
              (CallFunction|SetCartLeanState _leanamountneeded_2)
              (Variables|Default|SetCurrentLeanAmount _leanamountneeded_2)))
          (elif (and (not (Variables|Default|GetDebug_LeanLeft)) (not (Variables|Default|GetDebug_LeanRight)))
            (CallFunction|SetCartLeanState 0.0)
            (else
              (CallFunction|SetCartLeanState (Variables|Default|GetCurrentLeanAmount)))))))))

(event Collision|EventActorBeginOverlap
  (params (OtherActor :type Actor%20Object%20Reference))
  ;[1 1 1] Collison with track
  (if (Variables|JumpSettings|GetIsJumping)
    (bind _asbp_train_track (Utilities|Casting|CastToBP_TrainTrack OtherActor))
    (Variables|Default|SetAttachedTrack _asbp_train_track)
    (Physics|SetEnableGravity (Variables|Default|GetCarriageBodyMesh) false)
    (CallFunction|InitalizeTrainCarriage)
    (Variables|JumpSettings|SetIsJumping false)))

(event EventUpdateAnimations
  ;[1 1 1] Overwrite the update animation function for the mine cart since we are using a different anim blueprint
  (bind _asanimbp_mine_cart (Utilities|Casting|CastToANIMBP_MineCart (Components|SkeletalMesh|GetAnimInstance (Variables|Default|GetFrontBogieMesh))))
  (Variables|/Game/TrainAndRail/Models/MineCart/ANIMBP_MineCart.ANIMBP_MineCart_C|SetWheelSpeed _asanimbp_mine_cart (CallFunction|GetWheelSpeed)))

(event Input|ActionEvents|InputActionLeanLeft
  (params (Key :type Key%20Structure))
  (:Pressed
    (Variables|Default|SetDebug_LeanLeft true)
    (Variables|Default|SetJumpLeanFactor -2e+02))
  (:Released
    (Variables|Default|SetDebug_LeanLeft false)
    (Variables|Default|SetDebug_LeanRight false)
    (Variables|Default|SetJumpLeanFactor 0.0)))

(event Input|ActionEvents|InputActionLeanRight
  (params (Key :type Key%20Structure))
  (:Pressed
    (Variables|Default|SetDebug_LeanRight true)
    (Variables|Default|SetJumpLeanFactor 2e+02))
  (:Released
    (Variables|Default|SetDebug_LeanLeft false)
    (Variables|Default|SetDebug_LeanRight false)
    (Variables|Default|SetJumpLeanFactor 0.0)))

(event Input|KeyboardEvents|2
  (params (Key :type Key%20Structure))
  (:Pressed
    (Variables|Default|SetDebug_LeanLeft false)
    (Variables|Default|SetDebug_LeanRight false))
  (:Released
    (Variables|Default|SetDebug_LeanLeft false)
    (Variables|Default|SetDebug_LeanRight false)
    (Variables|Default|SetJumpLeanFactor 0.0)))

(event Input|KeyboardEvents|3
  (params (Key :type Key%20Structure))
  (:Pressed
    (Variables|Default|SetDebug_LeanRight true)
    (Variables|Default|SetJumpLeanFactor 2e+02))
  (:Released
    (Variables|Default|SetDebug_LeanLeft false)
    (Variables|Default|SetDebug_LeanRight false)
    (Variables|Default|SetJumpLeanFactor 0.0)))

(event Input|KeyboardEvents|1
  (params (Key :type Key%20Structure))
  (:Pressed
    (Variables|Default|SetDebug_LeanLeft true)
    (Variables|Default|SetJumpLeanFactor -2e+02))
  (:Released
    (Variables|Default|SetDebug_LeanLeft false)
    (Variables|Default|SetDebug_LeanRight false)
    (Variables|Default|SetJumpLeanFactor 0.0)))

(event Input|KeyboardEvents|E
  (params (Key :type Key%20Structure))
  (:Pressed
    (if (not (Variables|JumpSettings|GetIsJumping))
      (if (not (Variables|Default|GetIsRightHandleDown))
        (Variables|Default|SetIsRightHandleDown true)
        (CallFunction|ProcessInput 0.8)
        (if (Utilities|Enum|NotEqual(Enum) (Variables|Default|GetCarriageState) "NewEnumerator2")
          (CallFunction|ApplyPump 1.0))))))

(event Input|KeyboardEvents|SpaceBar
  (params (Key :type Key%20Structure))
  (:Pressed
    (if (not (Variables|JumpSettings|GetIsJumping))
      (CallFunction|StartJump))))

(event Input|KeyboardEvents|T
  (params (Key :type Key%20Structure)))

(event Input|KeyboardEvents|W
  (params (Key :type Key%20Structure))
  (:Pressed
    (if (not (Variables|JumpSettings|GetIsJumping))
      (if (Variables|Default|GetIsRightHandleDown)
        (Variables|Default|SetIsRightHandleDown false)
        (CallFunction|ProcessInput 0.2)
        (if (Utilities|Enum|NotEqual(Enum) (Variables|Default|GetCarriageState) "NewEnumerator2")
          (CallFunction|ApplyPump 1.0))))))

(fn ConstructionScript
  (|CallParentFunction))

(fn StartJump
  (bind _carriagebodymesh (Variables|Default|GetCarriageBodyMesh))
  (if (not (Variables|JumpSettings|GetIsJumping))
    (Variables|JumpSettings|SetIsJumping true)
    (Variables|Default|SetAttachedTrack 0)
    (Physics|SetEnableGravity _carriagebodymesh true)
    (Physics|SetPhysicsLinearVelocity _carriagebodymesh (+ (+ (Math|Vector|MakeVector 0.0 0.0 8e+02) (* (Transformation|GetActorForwardVector) (* 50 (Variables|Default|GetCurrentSpeed)))) (* (Transformation|GetActorRightVector) (Variables|Default|GetJumpLeanFactor))) false "None")))

(fn TickJump
  (params (DeltaSeconds :type Float%20%28single-precision%29%20%28by%20ref%29)))

(fn EndJump
  (Variables|JumpSettings|SetIsJumping false))

(fn SetJumpSettings
  (params (JumpDuration :type Float%20%28single-precision%29) (JumpTransform :type Transform))
  (Variables|JumpSettings|SetJumpRunTime JumpDuration)
  (Variables|JumpSettings|SetJumpTransform JumpTransform)
  (Variables|JumpSettings|SetJumpPeak (/ (Variables|JumpSettings|GetJumpRunTime) 2.0)))

(fn UpdateDynamicMass
  (LocalVariables|SetzDistance (- (.z (Transformation|GetWorldLocation (Variables|Default|GetFrontHitch))) (.z (Transformation|GetWorldLocation (Variables|Default|GetRearHitch)))))
  (LocalVariables|SetoutsideTolerance (>= (Math|Float|Absolute(Float) (LocalVariables|GetzDistance)) (LocalVariables|GetTolerance)))
  (if (> (LocalVariables|GetzDistance) 0.0)
    (if (LocalVariables|GetoutsideTolerance)
      (Variables|Default|SetMass 0.0))
    (elif (LocalVariables|GetoutsideTolerance)
      (Variables|Default|SetMass (Variables|Default|GetSavedMass)))))

(fn ProcessObstacle
  (params (Left :type Boolean) (Center :type Boolean) (Right :type Boolean) (LockoutTime :type Float%20%28single-precision%29)))

(fn SetCartLeanState
  (params (CurrentLean :type Float%20%28single-precision%29)))

(fn ProcessInput
  (params (CurrentHandleOffset :type Float%20%28single-precision%29))
  (LocalVariables|SetHandleOffset CurrentHandleOffset)
  (LocalVariables|SetHandleRotator (Variables|/Script/Engine.SceneComponent|GetRelativeRotation (Variables|Default|GetHandleParentTransform)))
  (Utilities|FlowControl|Sequence
    (:then_0
      ;[1 1 1] Animation Processing
      (bind _output_get (LocalVariables|SetAbsDistanceFromCenter (* (Math|Float|Absolute(Float) (- 0.5 (LocalVariables|GetHandleOffset))) 2.0)))
      (LocalVariables|SettargetRotation (* _output_get (LocalVariables|GetMaxAngle)))
      (if (<= (LocalVariables|GetHandleOffset) 0.5)
        _
        (else
          ;;[1 1 1] TargetAngle *=-1 to rotate in the right direction
          (LocalVariables|SettargetRotation (* (LocalVariables|GettargetRotation) -1.0))))
      ;;[1 1 1] Account for sensor jumps by ignoring large deltas
      (bind _output_get_2 (LocalVariables|SetSignedHandleDelta (- (Variables|InputVariables|GetLastHandlePosition) (LocalVariables|GetHandleOffset))))
      (bind _output_get_3 (Variables|InputVariables|SetLastHandlePosition (LocalVariables|GetHandleOffset)))
      (if (not (> (Math|Float|Absolute(Float) _output_get_2) 0.9))
        ;;[1 1 1] Rotate the handle
        (Variables|Default|SetLastValidDelta (- (LocalVariables|GettargetRotation) (.Pitch (Math|Rotator|BreakRotator (LocalVariables|GetHandleRotator)))))
        (Transformation|SetRelativeRotation (Variables|Default|GetHandleParentTransform) (Math|Rotator|MakeRotator (.Roll (Math|Rotator|BreakRotator (LocalVariables|GetHandleRotator))) (LocalVariables|GettargetRotation) (.Yaw (Math|Rotator|BreakRotator (LocalVariables|GetHandleRotator)))) false false)))
    (:then_1
      ;[1 1 1] Motion Processing
      ;;[1 1 1] Detect if the pumping direction changed
      (LocalVariables|SetSwitched%20Direction (Class|KismetMathLibrary|XORBoolean (and (<= (Variables|Default|GetLastValidDelta) 0.0) (not (Variables|Default|GetLastFramePumpDirection))) (and (> (Variables|Default|GetLastValidDelta) 0.0) (Variables|Default|GetLastFramePumpDirection))))
      (Variables|Default|SetLastFramePumpDirection (<= (Variables|Default|GetLastValidDelta) 0.0))
      ;;[1 1 1] Accumulate the pump distance
      (if (LocalVariables|GetSwitched%20Direction)
        ;;[1 1 1] Apply pump if enough angle difference is measured
        (if (> (Variables|Default|GettotalPumpDistance) 1e+01)
          (CallFunction|ApplyPump (Math|Float|Min(Float) (/ (Variables|Default|GettotalPumpDistance) (LocalVariables|GetMaxAngle)) (LocalVariables|GetMaxAngle))))
        (Variables|Default|SettotalPumpDistance 0.0)
        (else
          (Variables|Default|SettotalPumpDistance (+ (Variables|Default|GettotalPumpDistance) (Math|Float|Absolute(Float) (Variables|Default|GetLastValidDelta)))))))))

(fn CheckLeanStateforSparks
  (bind _output_get (LocalVariables|SetdeltaZ (- (.z (Transformation|GetWorldLocation (Variables|Default|GetRight%20Tracker))) (.z (Transformation|GetWorldLocation (Variables|Default|GetLeftTracker))))))
  (if (> (Math|Float|Absolute(Float) _output_get) (Variables|Default|GetLeanSparksActivateThreashold))
    (if (> (LocalVariables|GetdeltaZ) 0.0)
      (Components|Activation|Activate (Variables|Default|GetB_L_Sparks) false)
      (else
        (Components|Activation|Activate (Variables|Default|GetB_R_Sparks) false)))
    (else
      (Components|Activation|Deactivate (Variables|Default|GetB_R_Sparks)))))

(fn HandleGyroInput
  (CallFunction|AveragePumpValues)
  (CallFunction|ProcessInput (Variables|InputVariables|GetSmoothedCartPump)))

(fn IsLeanBeingHeld
  (params (CurrentLeanState :type Byte :default 0))
  ;[1 1 1] Require a new direction to be held before switching
  (LocalVariables|Setlocal_isHeld false)
  (if true
    (bind _result (Math|Integer|IncrementInt (Variables|Default|GetLeanTickCounter))
      (:%20%20
        (if (> _result (Variables|Default|GetnumberOfTicksToBeStable))
          (LocalVariables|Setlocal_isHeld true)
          (return (LocalVariables|Getlocal_isHeld)))))
    (else
      (Variables|Default|SetlastLeanState CurrentLeanState)
      (Variables|Default|SetLeanTickCounter 0)
      (LocalVariables|Setlocal_isHeld false)
      (return (LocalVariables|Getlocal_isHeld)))))

(fn AverageLeanValues
  ;[1 1 1] Add the current lean value up to a max of 20
  (Utilities|Array|Add (Variables|InputVariables|GetpreviousLeanValues) (Input|AxisValues|GetCartLean))
  (if (> (Utilities|Array|Length (Variables|InputVariables|GetpreviousLeanValues)) 15)
    (Utilities|Array|RemoveIndex (Variables|InputVariables|GetpreviousLeanValues))
    ;[1 1 1] Average  the previous 20 values of the lean
    (for _array_element (Variables|InputVariables|GetpreviousLeanValues)
      (LocalVariables|Setsum (+ (LocalVariables|Getsum) _array_element)))
    (Variables|Default|SetSmoothedCartLean (/ (LocalVariables|Getsum) (Math|Conversions|ToFloat(Integer) (Utilities|Array|Length (Variables|InputVariables|GetpreviousLeanValues)))))))

(fn AveragePumpValues
  ;[1 1 1] Add the current lean value up to a max
  (Utilities|Array|Add (Variables|InputVariables|GetpreviousPumpValues) (Input|AxisValues|GetHandleLean))
  (if (> (Utilities|Array|Length (Variables|InputVariables|GetpreviousPumpValues)) (LocalVariables|GetHowManyValuesToAverage))
    (Utilities|Array|RemoveIndex (Variables|InputVariables|GetpreviousPumpValues))
    ;[1 1 1] Average  the previous N values of the lean
    (for _array_element (Variables|InputVariables|GetpreviousPumpValues)
      (LocalVariables|SetSum (+ (LocalVariables|GetSum) _array_element)))
    (Variables|InputVariables|SetSmoothedCartPump (/ (LocalVariables|GetSum) (Math|Conversions|ToFloat(Integer) (Utilities|Array|Length (Variables|InputVariables|GetpreviousPumpValues)))))))

(fn ApplyPump
  (params (PumpStrength :type Float%20%28single-precision%29))
  (Variables|Default|SetPumpTimer (* PumpStrength (Variables|Default|GetBoostTimePerPump)))
  (Variables|Default|SetaveragePumpTime (/ (+ (Variables|Default|GetaveragePumpTime) (Variables|Default|GetTimeSinceLastPump)) 2.0))
  (Variables|Default|SetTimeSinceLastPump 0.0))

(fn HandleNonPlayerControl
  (bind _output_get (Variables|PlayerLockout|SetLockoutTimer (- (Variables|PlayerLockout|GetLockoutTimer) (Utilities|Time|GetWorldDeltaSeconds))))
  (if (<= _output_get 0.0)
    (CallFunction|ApplyorReleaseBrakes false)
    (Variables|PlayerLockout|SetPlayerControlLockout false)))

(fn StartRotateJump
  (bind _carriagebodymesh (Variables|Default|GetCarriageBodyMesh))
  (if (not (Variables|JumpSettings|GetIsJumping))
    (Variables|JumpSettings|SetIsJumping true)
    (Variables|Default|SetAttachedTrack 0)
    (Physics|SetEnableGravity _carriagebodymesh true)
    (Physics|SetPhysicsLinearVelocity _carriagebodymesh (+ (+ (Math|Vector|MakeVector 0.0 0.0 8e+02) (* (Transformation|GetActorForwardVector) (* (Math|Integer|SelectInt -50 50 (Variables|Default|GetInvertDir)) (Variables|Default|GetCurrentSpeed)))) (* (Transformation|GetActorRightVector) (Variables|Default|GetJumpLeanFactor))) false "None")
    (Class|PrimitiveComponent|SetPhysicsAngularVelocityinDegrees _carriagebodymesh "0, 0,100.000000" false "None")
    (bind _output_get (Variables|Default|SetInvertDir (not (Variables|Default|GetInvertDir))))
    (Development|PrintString (Utilities|String|ToString(Boolean) _output_get))))