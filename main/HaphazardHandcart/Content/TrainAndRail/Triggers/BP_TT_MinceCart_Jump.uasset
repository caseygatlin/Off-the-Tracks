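; Train-track trigger that makes a mine cart jump when it activates the trigger.
; On the internal trigger event it casts the carriage to BP_MineCart and ignores other carriage types.
; If the cart is not already jumping, it passes its jump duration and transform to the cart, then starts the jump.
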(event EventBeginPlay)

(event Collision|EventActorBeginOverlap
  (params (OtherActor :type Actor%20Object%20Reference)))

(event EventInternalTriggerEvent
  (params (Bogie :type AC%20Bogie%20Object%20Reference) (Carriage :type BP%20Train%20Carriage%20Object%20Reference))
  ;[1 1 1] If fired by a mine cart and it's not already jumping, setup the jump and make it happen
  (bind _asbp_mine_cart (Utilities|Casting|CastToBP_MineCart Carriage))
  (if (not (Variables|/Game/TrainAndRail/Trains/BP_MineCart.BP_MineCart_C|GetIsJumping _asbp_mine_cart))
    (Default|SetJumpSettings _asbp_mine_cart (Variables|JumpSettings|GetJumpDuration) (Variables|JumpSettings|GetJumpTransform))
    (Default|StartJump _asbp_mine_cart)))

(event EventTick
  (params (DeltaSeconds :type Float%20%28single-precision%29))
  (|CallParentFunction 0.0))

(fn ConstructionScript
  (|CallParentFunction))