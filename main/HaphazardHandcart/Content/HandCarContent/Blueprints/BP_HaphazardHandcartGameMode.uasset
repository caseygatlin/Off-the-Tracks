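; Game mode Blueprint for Haphazard Handcart that runs the player HUD and the end-of-level flow.
; BeginPlay adds the HUD, loads or creates the high-score save and finds the score billboard.
; When Tick sees HUD progress complete, it scores time and collectibles, saves and shows the end screen.
; After a delay the billboard prompts pumping, and strong handcart input opens the configured level; second-HUD logic is unwired.
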(event EventBeginPlay
  ;[1 1 1] Creates HUD and Initializes
  (bind _returnvalue (UserInterface|CreateWidget "/Game/HandCarContent/UI/Widgets/HUD.HUD_C" (Game|GetPlayerController 0)))
  (bind _output_get (Variables|UI|Set1PlayerHUD _returnvalue))
  (UserInterface|Viewport|AddtoViewport _output_get 0)
  (CallFunction|LoadGame)
  (bind _returnvalue_2 (Actor|GetActorOfClass "/Game/HandCarContent/Blueprints/BP_ScoreBillboard.BP_ScoreBillboard_C"))
  (Variables|UI|SetScoreBillboard _returnvalue_2))

(event EventTick
  (params (DeltaSeconds :type Float%20%28single-precision%29))
  (bind _savegame (Variables|Default|GetSaveGame))
  (Utilities|FlowControl|Sequence
    (:then_0
      ;[1 1 1] Distance traveled
      (bind _ashaphazard_handcart_game_mode (Utilities|Casting|CastToHaphazardHandcartGameMode (Game|GetGameMode))))
    (:then_1
      ;[1 1 1] (HUD 1) Setting up End Level Screen
      (if (== (Variables|/Game/HandCarContent/UI/Widgets/HUD.HUD_C|GetCurrentProgress (Variables|UI|Get1PlayerHUD)) 1.0)
        (Utilities|FlowControl|DoOnce false
          (:Completed
            (Viewport|RemoveAllWidgets)
            (bind _returnvalue (UserInterface|CreateWidget "/Game/HandCarContent/UI/Widgets/EndLevel.EndLevel_C" (Game|GetPlayerController 0)))
            (Variables|UI|SetEndLevelHUD _returnvalue)
            (bind _output_get (Variables|/Game/HandCarContent/UI/Widgets/EndLevel.EndLevel_C|SetFinalSeconds (Variables|UI|GetEndLevelHUD) (Variables|/Game/HandCarContent/UI/Widgets/HUD.HUD_C|GetSeconds (Variables|UI|Get1PlayerHUD))))
            (bind _output_get_2 (Variables|/Game/HandCarContent/UI/Widgets/EndLevel.EndLevel_C|SetFinalMinutes (Variables|UI|GetEndLevelHUD) (Variables|/Game/HandCarContent/UI/Widgets/HUD.HUD_C|GetMinutes (Variables|UI|Get1PlayerHUD))))
            (bind _score (CallFunction|CalculateScore _output_get _output_get_2))
            (bind _output_get_3 (Variables|/Game/HandCarContent/UI/Widgets/EndLevel.EndLevel_C|SetFinalScore (Variables|UI|GetEndLevelHUD) _score))
            (Class|SaveHighScore|SaveHighScore _savegame _output_get_3)
            (Variables|/Game/HandCarContent/UI/Widgets/EndLevel.EndLevel_C|SetHighScores (Variables|UI|GetEndLevelHUD) (Class|SaveHighScore|GetHighScores _savegame))
            (UserInterface|Viewport|AddtoViewport (Variables|UI|GetEndLevelHUD) 0)
            (Utilities|FlowControl|Delay (Variables|Default|GetContinueDelay))
            (Default|PumptoContinueAnim (Variables|UI|GetScoreBillboard))
            (Variables|Default|SetCanContinue true)))))
    (:then_2
      ;[1 1 1] If can continue, then check for pumping
      (if (Variables|Default|GetCanContinue)
        (if (> (Math|Float|Absolute(Float) (Class|PlayerHandcar|GetInputAxis (Class|HaphazardHandcartGameMode|GetPlayerHandcar))) 0.5)
          (Variables|Default|SetCanContinue false)
          (Viewport|RemoveAllWidgets)
          (Game|OpenLevel(byName) (Utilities|String|StringToName (Variables|Default|GetSceneName))))))))

(fn ConstructionScript)

(fn CalculateScore
  (params (Seconds :type Integer) (Minutes :type Integer))
  (return (+ (* (+ Seconds (* Minutes 60)) 87) (* (Class|HaphazardHandcartGameMode|GetNumCollectibles) 200))))

(fn LoadGame
  (bind _returnvalue (SaveGame|DoesSaveGameExist (Variables|Default|GetSlotName) (Variables|Default|GetUserIndex)))
  (if _returnvalue
    (bind _returnvalue_2 (SaveGame|LoadGamefromSlot (Variables|Default|GetSlotName) (Variables|Default|GetUserIndex)))
    (bind _asbp_save_high_score (Utilities|Casting|CastToBP_SaveHighScore _returnvalue_2))
    (Variables|Default|SetSaveGame _asbp_save_high_score)
    (else
      (bind _returnvalue_3 (SaveGame|CreateSaveGameObject "/Game/HandCarContent/Blueprints/BP_SaveHighScore.BP_SaveHighScore_C"))
      (Variables|Default|SetSaveGame _returnvalue_3))))