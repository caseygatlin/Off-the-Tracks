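; Player handcar that animates its two riders pumping and drives a speed visual effect while boosting.
; Each tick, UpdatePP eases the "Visibility" scalar in the PC_Speed material parameter collection toward on or off based on boost state.
; UpdatePlayerAnim turns normalized pump input into arm rotation and translation offsets on each rider's GirlAnim instance, with opposite pump signs so the two riders move in opposition.
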(event EventBeginPlay)

(event Collision|EventActorBeginOverlap
  (params (OtherActor :type Actor%20Object%20Reference)))

(event EventTick
  (params (DeltaSeconds :type Float%20%28single-precision%29))
  (CallFunction|UpdatePP)
  ;[1 1 1] Update arm offsets for characters
  (CallFunction|UpdatePlayerAnim (Variables|Default|GetPlayer%201) -1.0)
  (CallFunction|UpdatePlayerAnim (Variables|Default|GetPlayer%202) 1.0))

(fn ConstructionScript)

(fn UpdatePP
  (if (Class|PlayerHandcar|GetCartBoostState)
    (LocalVariables|SetLerpTarget 1.0)
    (else
      (LocalVariables|SetLerpTarget 0.0)))
  (bind _returnvalue (Rendering|Material|GetScalarParameterValue "/Game/HandCarContent/Materials/Master/PC_Speed.PC_Speed" "Visibility" :!class /Script/Engine.KismetMaterialLibrary))
  (LocalVariables|SetCurrentSpeed _returnvalue)
  (Rendering|Material|SetScalarParameterValue "/Game/HandCarContent/Materials/Master/PC_Speed.PC_Speed" "Visibility" (Math|Interpolation|FInterptoConstant (LocalVariables|GetCurrentSpeed) (LocalVariables|GetLerpTarget) (Utilities|Time|GetWorldDeltaSeconds) 1.3) :!class /Script/Engine.KismetMaterialLibrary))

(fn UpdatePlayerAnim
  (params (Player :type Skeletal%20Mesh%20Component%20Object%20Reference%20%28by%20ref%29) (PumpSign :type Float%20%28single-precision%29))
  (bind _returnvalue (Input|AxisValues|GetNormalCtrl_Pump))
  (bind _returnvalue_2 (Math|Float|Absolute(Float) _returnvalue))
  (bind _returnvalue_3 (* _returnvalue_2 6.7))
  (bind _returnvalue_4 (* _returnvalue_2 6.1))
  (bind _returnvalue_5 (+ _returnvalue_3 -34.5))
  (bind _returnvalue_6 (+ _returnvalue_4 -44.5))
  ;[1 1 1] Apply offsets to arms of character
  (Variables|Default|SetPumpSign PumpSign)
  (bind _asgirl_anim (Utilities|Casting|CastToGirlAnim (Components|SkeletalMesh|GetAnimInstance Player)))
  (Variables|/Game/HandCarContent/Geometry/Character/GirlAnim.GirlAnim_C|SetLeftArmPump _asgirl_anim (Math|Rotator|MakeRotator (- (* _returnvalue 28.0 (Variables|Default|GetPumpSign)) (+ (* _returnvalue 2.2) 7.9)) _returnvalue_5 _returnvalue_6))
  (Variables|/Game/HandCarContent/Geometry/Character/GirlAnim.GirlAnim_C|SetRightArmPump _asgirl_anim (Math|Rotator|MakeRotator (- (* _returnvalue 28.0 (Variables|Default|GetPumpSign)) (+ (* _returnvalue 2.2) 7.9)) (* _returnvalue_5 -1.0) (* _returnvalue_6 -1.0)))
  (Variables|/Game/HandCarContent/Geometry/Character/GirlAnim.GirlAnim_C|SetRightArmTranslation _asgirl_anim (Math|Vector|MakeVector (* (Math|Float|Absolute(Float) (Input|AxisValues|GetNormalCtrl_Pump)) 1.2) 0.0 0.0))
  (Variables|/Game/HandCarContent/Geometry/Character/GirlAnim.GirlAnim_C|SetLeftArmTranslation _asgirl_anim (Math|Vector|MakeVector (* (Math|Float|Absolute(Float) (Input|AxisValues|GetNormalCtrl_Pump)) -1.2) 0.0 0.0)))