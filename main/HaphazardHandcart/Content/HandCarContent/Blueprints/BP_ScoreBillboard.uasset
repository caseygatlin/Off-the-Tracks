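; BP_ScoreBillboard is a score billboard actor that shows an animated continue text prompt.
; The construction script hides ContinueText, and PumpToContinueAnim reveals it after a zero-length delay and drives its world size with a timeline.
; CountDownAnim is empty, and the timeline and timer logic for counting down EndLevel's final minutes and seconds is disconnected, so it never runs.
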(event Custom|PumpToContinueAnim
  (Utilities|FlowControl|Delay 0.0)
  (Rendering|SetVisibility (Variables|Default|GetContinueText) true false)
  (bind _world_size (Timeline|Timeline_0 Play)
    (:Update
      (Rendering|Components|TextRender|SetWorldSize (Variables|Default|GetContinueText) _world_size))))

(event Custom|CountDownAnim)

(event EventBeginPlay)

(event Collision|EventActorBeginOverlap
  (params (OtherActor :type Actor%20Object%20Reference)))

(event EventTick
  (params (DeltaSeconds :type Float%20%28single-precision%29)))

(fn ConstructionScript
  (Rendering|SetVisibility (Variables|Default|GetContinueText) false false))